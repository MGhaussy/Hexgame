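; Actor component that drives runtime hex grid building, spawning or reusing a HexGrid_RuntimeMapMaker and toggling build mode.
; Event dispatchers route tile clicks, mesh changes, activation and save/load to the grid, with loading first destroying the old one.
; While active, Tick traces the Camera channel from camera or cursor to update the hit tile's preview and feed the hit location to the GhostTiles material parameter collection.
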(event Custom|ActivateGridBuilderMode
  (params (SpawnTransform :type Transform))
  ;[1 1 1] Activate grid builder mode - spawns the grid
  (Variables|Default|GetGridBuilder ; If this is valid, we use the previous grid. If you want to support multiple grids, then remove this and always spawn
    (:then
      _)
    (:else
      (bind _returnvalue (Game|SpawnActorfromClass "/HexGrids/HexGrids/Blueprints/RuntimeGridManipulation/HexGrid_RuntimeMapMaker.HexGrid_RuntimeMapMaker_C" SpawnTransform "Undefined" (Components|GetOwner) (Variables|Default|GetMaxGridBuilderSize) (Variables|Default|GetGridScale) 0))
      (Variables|Default|SetGridBuilder _returnvalue)))
  ;[1 1 1] Enable system bool, enable tick, and call enable on the grid builder
  (Variables|Default|SetbMapBuilder true)
  (Components|Tick|SetComponentTickEnabled true)
  (Default|CallEnableGridBuilding (Variables|Default|GetGridBuilder)))

(event Custom|ClearOldGridAndReset
  ;[1 1 1] Delete Old Grid
  (Default|CallDeactivateGridBuilder)
  (bind _gridbuilder (Variables|Default|GetGridBuilder)
    (:then
      (Actor|DestroyActor _gridbuilder))
    (:else)))

(event Custom|SaveGrid_Internal
  (params (SlotName :type String) (UserIndex :type Integer))
  ;[1 1 1] Save Grid
  (bind _gridbuilder (Variables|Default|GetGridBuilder)
    (:then
      (Default|SaveGrid _gridbuilder SlotName UserIndex)
      (Development|PrintString "Saving Grid"))
    (:else)))

(event Custom|TileInteraction_Internal
  ;[1 1 1] On Tile interaction, inform grid
  (if (Variables|Default|GetbMapBuilder)
    (Default|TileAction (Variables|Default|GetGridBuilder))))

(event Custom|ChangePlacedMesh_Internal
  (params (NextMesh :type Static%20Mesh%20Object%20Reference))
  ;[1 1 1] Change Mesh to spawn
  (Variables|/HexGrids/HexGrids/Blueprints/RuntimeGridManipulation/HexGrid_RuntimeMapMaker.HexGrid_RuntimeMapMaker_C|SetMeshToSpawn (Variables|Default|GetGridBuilder) NextMesh))

(event Custom|LoadGrid_Internal
  (params (SlotName :type String) (UserIndex :type Integer))
  ;[1 1 1] Load Grid
  (CallFunction|ClearOldGridandReset)
  (Default|CallActivateGridBuilderSystem)
  (Variables|/HexGrids/HexGrids/Blueprints/RuntimeGridManipulation/HexGrid_RuntimeMapMaker.HexGrid_RuntimeMapMaker_C|SetLoadExistingGridFromSave (Variables|Default|GetGridBuilder) true)
  (Default|LoadGrid (Variables|Default|GetGridBuilder) SlotName UserIndex)
  (Development|PrintString "Loading Grid"))

(event Custom|DeactivateGridBuilderMode
  ;[1 1 1] Deactivate the grid. Stops the ticking, and passes stop into the grid
  (Variables|Default|SetbMapBuilder false)
  (Components|Tick|SetComponentTickEnabled false)
  (bind _gridbuilder (Variables|Default|GetGridBuilder)
    (:then
      (Default|CallDisableGridBuilding _gridbuilder))
    (:else)))

(event EventBeginPlay
  ;[1 1 1] If your using a pawn, you could dump this. The char ref is only for the demo stuff, and not required to make this work.
  (bind _ascharacter (Utilities|Casting|CastToCharacter (Components|GetOwner))
    (:then
      (Variables|Default|SetCharacterRef _ascharacter))
    (:CastFailed
      _))
  ;[1 1 1] This is the event dispatcher we call on click
  (EventDispatchers|BindEventtoTileInteraction (EventDispatchers|CreateEvent :!event Custom|TileInteraction_Internal))
  ;[1 1 1] And these are the dispatchers we call to activate/deactivate the system
  (EventDispatchers|BindEventtoActivateGridBuilderSystem (EventDispatchers|CreateEvent :!event Custom|ActivateGridBuilderMode))
  (EventDispatchers|BindEventtoDeactivateGridBuilder (EventDispatchers|CreateEvent :!event Custom|DeactivateGridBuilderMode))
  ;[1 1 1] These dispatchers call the load and save systems
  (EventDispatchers|BindEventtoLoadGridfromFile (EventDispatchers|CreateEvent :!event Custom|LoadGrid_Internal))
  (EventDispatchers|BindEventtoSaveGridtoFile (EventDispatchers|CreateEvent :!event Custom|SaveGrid_Internal))
  ;[1 1 1] update placed mesh
  (EventDispatchers|BindEventtoChangePlacedMesh (EventDispatchers|CreateEvent :!event Custom|ChangePlacedMesh_Internal)))

(event EventTick
  (params (DeltaSeconds :type Float%20%28single-precision%29))
  (bind _returnvalue (Game|GetPlayerCameraManager 0))
  (bind _returnvalue_2 (Camera|GetCameraLocation _returnvalue))
  ;[1 1 1] On Tick
  (if (Variables|Default|GetbMapBuilder)
    ;[1 0 0.02781 1 14] !IMPORTANT!
    ; Here we perform the line trace. Right now we are using the camera trace channel, but for best results, you should make a custom trace channel in the project settings.
    ; Custom trace channels get stored in the project ini's, so I cannot include it in the plugin.
    ; Once you do that, update the meshes to react to that. Block it on the ghost instanceStaticMeshComponent (in RuntimeMapBuilder Blueprint), and ignore it on the placed static mesh components (Also in RuntimeMapBuilder). Also the hit results under cursor has no ignore self, so it hits the player character capsule, so set that trace as well to ignore your custom trace channel
    (bind _outhit (Collision|LineTraceByChannel _returnvalue_2 (+ _returnvalue_2 (* (Math|Vector|GetForwardVector (Variables|/Script/Engine.PlayerCameraManager|GetTransformComponent _returnvalue)) 2e+03)) "TraceTypeQuery2" false 0 "None"))
    ;[1 1 1] Uses the tick to update the preview mesh. We also used the hitItem to control where actual spawns happen.
    (if (.bBlockingHit (Collision|BreakHitResult (select (Variables|Default|GetUseMouseCursorForTrace) (.HitResult (Game|Player|GetHitResultUnderCursorbyChannel (Game|GetPlayerController 0) "TraceTypeQuery2" false)) _outhit)))
      (if (== (.HitActor (Collision|BreakHitResult (select (Variables|Default|GetUseMouseCursorForTrace) (.HitResult (Game|Player|GetHitResultUnderCursorbyChannel (Game|GetPlayerController 0) "TraceTypeQuery2" false)) _outhit))) (Variables|Default|GetGridBuilder))
        (Utilities|FlowControl|Sequence
          (:then_0
            (Default|UpdatePreview (Variables|Default|GetGridBuilder) (.HitItem (Collision|BreakHitResult (select (Variables|Default|GetUseMouseCursorForTrace) (.HitResult (Game|Player|GetHitResultUnderCursorbyChannel (Game|GetPlayerController 0) "TraceTypeQuery2" false)) _outhit)))) ; Pass the hit instance ID
          )
          (:then_1
            (Rendering|Material|SetVectorParameterValue "/HexGrids/HexGrids/Materials/GhostTiles.GhostTiles" "MouseTraceLocWS" (Math|Conversions|ToLinearColor(Vector) (.Location (Collision|BreakHitResult (select (Variables|Default|GetUseMouseCursorForTrace) (.HitResult (Game|Player|GetHitResultUnderCursorbyChannel (Game|GetPlayerController 0) "TraceTypeQuery2" false)) _outhit)))) :!class /Script/Engine.KismetMaterialLibrary) ; Update the hit location in the ghost material
          ))))))