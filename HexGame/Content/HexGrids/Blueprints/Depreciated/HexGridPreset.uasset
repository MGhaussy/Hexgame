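; HexGridPreset, filed as deprecated, builds a hex tile grid in a selectable rectangle, hexagon, triangle or parallelogram shape.
; Its Spawn event clears old instances, optionally derives X scale from Y for perfect hexagons, then generates the tile array.
; Each tile is scaled and offset into hex layout as a flat instanced static mesh instance, with its index recorded in InstanceMap for lookup by tile.
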(event Custom|Spawn
  (bind _gridscale (Variables|Default|GetGridScale))
  (bind _gridsize (Variables|Default|GetGridSize))
  ;[1 1 1] Clean Up Old
  (Components|InstancedStaticMesh|ClearInstances (Variables|Default|GetInstancedStaticMesh))
  (Utilities|Array|Clear (Variables|Default|GetGrid))
  (Utilities|IsValid (Variables|Default|GetInstancedStaticMesh)
    (:Is%20Valid
      (Utilities|FlowControl|Sequence
        (:then_0
          ;[1 1 1] For perfect spacing, calculate the X based off the Y when using perfect hexagons
          (Variables|Default|SetGridScaleCalculated (select (Variables|Default|GetCalculateGridXScale) (Math|Vector|MakeVector (Class|GridsHex|HexWidth (.y _gridscale)) (.y _gridscale) (.z _gridscale)) (Variables|Default|GetGridScale))))
        (:then_1
          ;[1 1 1] Choose your grid shape, and build the grid
          (switch Utilities|FlowControl|Switch|SwitchonEHexGridShape (Variables|Default|GetShape)
            (:HexGrids_Rectangle
              (bind _returnvalue (Class|GridsHex|BuildRectangleArray _gridsize (Variables|Default|GetCenterGrid)))
              (Variables|Default|SetGrid _returnvalue))
            (:HexGrids_Hexagon
              (bind _returnvalue_2 (Class|GridsHex|BuildHexagonArray _gridsize))
              (Variables|Default|SetGrid _returnvalue_2))
            (:HexGrids_Triangle
              (bind _returnvalue_3 (Class|GridsHex|BuildTriangleArray _gridsize))
              (Variables|Default|SetGrid _returnvalue_3))
            (:HexGrids_Parallelogram
              (bind _returnvalue_4 (Class|GridsHex|BuildParallelogramArray _gridsize (Variables|Default|GetCenterGrid)))
              (Variables|Default|SetGrid _returnvalue_4)))
          (for _array_element (Variables|Default|GetGrid)
            ;[1 1 1] Scale the grid and offset into a hexagonal shape, and add instance
            (bind _returnvalue_5 (Components|InstancedStaticMesh|AddInstance (Variables|Default|GetInstancedStaticMesh) (Math|Conversions|ToTransform(Vector) (Math|Conversions|ToVector(Vector2D) (.Precise (Class|GridsHex|ScaleandOffset _array_element (Math|Conversions|ToVector2D(Vector) (Variables|Default|GetGridScaleCalculated))))))))
            (Utilities|Map|Add (Variables|Default|GetInstanceMap) _array_element _returnvalue_5)))))))