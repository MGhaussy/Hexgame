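; Fire-and-forget component that animates a static mesh's scale toward a target, with each instance running independently.
; BeginPlay waits one frame for expose-on-spawn variables, stores the start scale, then opens a gate on Tick.
; Tick interpolates the relative scale with VInterpTo until it is within tolerance of the target.
; It then closes the gate, fires a completion dispatcher, optionally destroys the mesh and destroys itself.
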(event Custom|CloseTickGate
  (bind _returnvalue (Utilities|Time|GetWorldDeltaSeconds))
  (bind _staticmeshcomponent (Variables|Default|GetStaticMeshComponent))
  (bind _targetscale (Variables|Default|GetTargetScale))
  (bind _scalespeed (Variables|Default|GetScaleSpeed))
  (bind _relativescale3d (Variables|/Script/Engine.SceneComponent|GetRelativeScale3D _staticmeshcomponent))
  (bind _returnvalue_2 (Math|Interpolation|VInterpTo _relativescale3d _targetscale _returnvalue _scalespeed))
  ;[0 0 0 0.5] This component allows you to animate the  scale of a static mesh, so you can loop through and perform the scale. Each one plays out independantly. The component is fire and forget, destroying itself once complete
  (Utilities|FlowControl|Gate true) ; enters at Close
)

(event Custom|OpenTickGate
  (bind _returnvalue (Utilities|Time|GetWorldDeltaSeconds))
  (bind _staticmeshcomponent (Variables|Default|GetStaticMeshComponent))
  (bind _targetscale (Variables|Default|GetTargetScale))
  (bind _scalespeed (Variables|Default|GetScaleSpeed))
  (bind _relativescale3d (Variables|/Script/Engine.SceneComponent|GetRelativeScale3D _staticmeshcomponent))
  (bind _returnvalue_2 (Math|Interpolation|VInterpTo _relativescale3d _targetscale _returnvalue _scalespeed))
  ;[0 0 0 0.5] This component allows you to animate the  scale of a static mesh, so you can loop through and perform the scale. Each one plays out independantly. The component is fire and forget, destroying itself once complete
  (Utilities|FlowControl|Gate true) ; enters at Open
)

(event EventBeginPlay
  ;[0 0 0 0.5] This component allows you to animate the  scale of a static mesh, so you can loop through and perform the scale. Each one plays out independantly. The component is fire and forget, destroying itself once complete
  (Utilities|FlowControl|Delay 0.0) ; Expose on spawn variables do not get always set in time, so a 1 frame delay fixes this
  (bind _staticmeshcomponent (Variables|Default|GetStaticMeshComponent)
    (:then
      (Variables|Default|SetStartScale (Variables|/Script/Engine.SceneComponent|GetRelativeScale3D _staticmeshcomponent)) ; Store Start Scale
      (CallFunction|OpenTickGate))
    (:else)))

(event EventTick
  (params (DeltaSeconds :type Float%20%28single-precision%29))
  (bind _returnvalue (Utilities|Time|GetWorldDeltaSeconds))
  (bind _staticmeshcomponent (Variables|Default|GetStaticMeshComponent))
  (bind _targetscale (Variables|Default|GetTargetScale))
  (bind _scalespeed (Variables|Default|GetScaleSpeed))
  (bind _relativescale3d (Variables|/Script/Engine.SceneComponent|GetRelativeScale3D _staticmeshcomponent))
  (bind _returnvalue_2 (Math|Interpolation|VInterpTo _relativescale3d _targetscale _returnvalue _scalespeed))
  ;[0 0 0 0.5] This component allows you to animate the  scale of a static mesh, so you can loop through and perform the scale. Each one plays out independantly. The component is fire and forget, destroying itself once complete
  (Utilities|FlowControl|Gate true ; Allow tick once variables start and target have been saved
    (:Exit
      (Transformation|SetRelativeScale3D (Variables|Default|GetStaticMeshComponent) _returnvalue_2)
      (if (Math|Vector|Equal(Vector) _returnvalue_2 (Variables|Default|GetTargetScale) 0.01) ; self destroy once interp has completed
        (CallFunction|CloseTickGate)
        (Default|CallScaleComplete) ; Optional dispatcher if needed
        (Utilities|FlowControl|Sequence
          (:then_0
            (if (Variables|Default|GetDestroyAffectedMeshOnComplete)
              (bind _staticmeshcomponent_2 (Variables|Default|GetStaticMeshComponent)
                (:then
                  (Components|DestroyComponent _staticmeshcomponent_2))
                (:else))))
          (:then_1
            (Components|DestroyComponent)))))))