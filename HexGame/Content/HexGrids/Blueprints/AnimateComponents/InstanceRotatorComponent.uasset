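; Fire-and-forget component that flips one hex-grid ISM instance 180 degrees, so each instance animates independently.
; After a one-frame delay it picks a rotation axis from a hex neighbour direction, using either the first diagonal-capable A* step toward the target (optionally inverted) or the target tile directly.
; A gated Tick interpolates the angle at constant speed, updates the instance transform, then destroys the component on completion.
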(event Custom|CloseSystem
  (bind _instanceref (Variables|Default|GetInstanceRef))
  (bind _instanceid (Variables|OnSpawnValues|GetInstanceID))
  (bind _outinstancetransform (Components|InstancedStaticMesh|GetInstanceTransform _instanceref _instanceid false))
  (bind (_location _rotation _scale) (Math|Transform|BreakTransform _outinstancetransform))
  ;[0 0 0 0] This component allows you to instance the animation of each ISM instance, so you can loop through and perform a rotation and each plays out independantly. The component is fire and forget, destroying itself once complete
  ;;[0 0 0] On Tick, Performs a rotator from axis and angle, finterps it from 0-180 on the angle, and updates the instance transform
  (Utilities|FlowControl|Gate true) ; enters at Close
)

(event Custom|EnableTick
  (bind _instanceref (Variables|Default|GetInstanceRef))
  (bind _instanceid (Variables|OnSpawnValues|GetInstanceID))
  (bind _outinstancetransform (Components|InstancedStaticMesh|GetInstanceTransform _instanceref _instanceid false))
  (bind (_location _rotation _scale) (Math|Transform|BreakTransform _outinstancetransform))
  ;[0 0 0 0] This component allows you to instance the animation of each ISM instance, so you can loop through and perform a rotation and each plays out independantly. The component is fire and forget, destroying itself once complete
  ;;[0 0 0] On Tick, Performs a rotator from axis and angle, finterps it from 0-180 on the angle, and updates the instance transform
  (Utilities|FlowControl|Gate true) ; enters at Open
)

(event EventBeginPlay
  (bind _returnvalue (Class|GridsHex|RotateTowardsNeighbourorDiagonalHex))
  (bind _currenttile (Variables|Default|GetCurrentTile))
  (bind _targettile (Variables|Default|GetTargetTile))
  (bind _direction (Class|GridsHex|FindNeighbourfromAdjacentOffsets _currenttile _targettile false))
  ;[0 0 0 0] This component allows you to instance the animation of each ISM instance, so you can loop through and perform a rotation and each plays out independantly. The component is fire and forget, destroying itself once complete
  (Utilities|FlowControl|Delay 0.0) ; Instance Ref Expose on spawn does not reliably get set on same frame\n1 frame offset corrects this
  (if (Variables|OnSpawnValues|GetOriginFacing)
    ;;[0 0 0] If Origin Facing, Uses Pathfinding (With diagonal support) to find a route to the origin, then gets the first step on the path, and decides what neighbour/diagonal direction that is. If it fails to find a direction (IE origin to origin, the first tile), uses a fallback direction. Invert vector gives the option to rotate away from the target, rather than towards it,
    (bind _results (Class|GridsHex|AStarPathfinding :StartPoint (Variables|Default|GetCurrentTile) :EndPoint (Variables|Default|GetTargetTile) :Grid (Variables|Default|GetGrid) :Cost (Variables|Default|GetCostFiller) :Blocked (Variables|Default|GetBlockedFiller) :bAllowInexact true :bAllowDiagonal true))
    (Variables|Default|SetRotatorAxis (Math|Vector|SelectVector (Utilities|Array|Get(acopy) _returnvalue (select (!= (.Direction (Class|GridsHex|FindNeighbourfromAdjacentOffsets (Variables|Default|GetCurrentTile) (Class|GridsCore|ToOffset(Cube) (Utilities|Array|Get(acopy) _results)) true)) -1) (.Direction (Class|GridsHex|FindNeighbourfromAdjacentOffsets (Variables|Default|GetCurrentTile) (Class|GridsCore|ToOffset(Cube) (Utilities|Array|Get(acopy) _results)) true)) 6)) (Class|GridsCore|InvertVector (Utilities|Array|Get(acopy) _returnvalue (select (!= (.Direction (Class|GridsHex|FindNeighbourfromAdjacentOffsets (Variables|Default|GetCurrentTile) (Class|GridsCore|ToOffset(Cube) (Utilities|Array|Get(acopy) _results)) true)) -1) (.Direction (Class|GridsHex|FindNeighbourfromAdjacentOffsets (Variables|Default|GetCurrentTile) (Class|GridsCore|ToOffset(Cube) (Utilities|Array|Get(acopy) _results)) true)) 6))) (Variables|OnSpawnValues|GetFlipTowardsTarget)))
    (else
      ;;[0 0 0] If not using origin facing, will instead use the target tile as its rotator orientation. You could also pass in any tile, but it must be adjacent to origin
      (Variables|Default|SetRotatorAxis (Utilities|Array|Get(acopy) _returnvalue (select (!= _direction -1) _direction 6)))))
  ;;[0 0 0] Stores default rotation, and the desired rotation, then allows tick to begin
  (bind _output_get (Variables|Default|SetStartRotation (.rotation (.OutInstanceTransform (Components|InstancedStaticMesh|GetInstanceTransform (Variables|Default|GetInstanceRef) (Variables|OnSpawnValues|GetInstanceID) false)))))
  (Variables|Default|SetDesiredRotation (Math|Rotator|CombineRotators _output_get (Math|Vector|RotatorfromAxisandAngle (Variables|Default|GetRotatorAxis) 1.8e+02)))
  (CallFunction|EnableTick))

(event EventTick
  (params (DeltaSeconds :type Float%20%28single-precision%29))
  (bind _instanceref (Variables|Default|GetInstanceRef))
  (bind _instanceid (Variables|OnSpawnValues|GetInstanceID))
  (bind _outinstancetransform (Components|InstancedStaticMesh|GetInstanceTransform _instanceref _instanceid false))
  (bind (_location _rotation _scale) (Math|Transform|BreakTransform _outinstancetransform))
  ;[0 0 0 0] This component allows you to instance the animation of each ISM instance, so you can loop through and perform a rotation and each plays out independantly. The component is fire and forget, destroying itself once complete
  ;;[0 0 0] On Tick, Performs a rotator from axis and angle, finterps it from 0-180 on the angle, and updates the instance transform
  (Utilities|FlowControl|Gate true
    (:Exit
      (Variables|Default|SetFInterpProgress (Math|Interpolation|FInterptoConstant (Variables|Default|GetFInterpProgress) 1.8e+02 (Utilities|Time|GetWorldDeltaSeconds) (Variables|OnSpawnValues|GetInterpSpeed)))
      (Components|InstancedStaticMesh|UpdateInstanceTransform (Variables|Default|GetInstanceRef) (Variables|OnSpawnValues|GetInstanceID) (Math|Transform|MakeTransform _location (Math|Rotator|CombineRotators (Variables|Default|GetStartRotation) (Math|Vector|RotatorfromAxisandAngle (Variables|Default|GetRotatorAxis) (Variables|Default|GetFInterpProgress))) _scale) false true true)
      ;;[0 0 0] When FInterp has completed its move, this component is no longer required. shuts down the tick then destroys self
      (if (Math|Rotator|Equal(Rotator) (Math|Rotator|CombineRotators (Variables|Default|GetStartRotation) (Math|Vector|RotatorfromAxisandAngle (Variables|Default|GetRotatorAxis) (Variables|Default|GetFInterpProgress))) (Variables|Default|GetDesiredRotation) 0.01)
        (CallFunction|CloseSystem)
        (Components|DestroyComponent)))))