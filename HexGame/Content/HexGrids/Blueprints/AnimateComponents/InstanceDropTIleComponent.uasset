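; Fire-and-forget component that animates a single instanced static mesh instance dropping vertically, so many hex tile instances can each fall independently.
; After a one-frame delay for expose-on-spawn values, it stores the start location and a target lowered by the drop height.
; A gated Tick moves the instance toward the target with VInterpTo.
; On arrival it closes the gate, fires a move-complete dispatcher and destroys itself.
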(event Custom|CloseTickGate
  (bind _returnvalue (Utilities|Time|GetWorldDeltaSeconds))
  (bind _instanceid (Variables|Default|GetInstanceID))
  (bind _instancecomponent (Variables|Default|GetInstanceComponent))
  (bind _targetlocation (Variables|Default|GetTargetLocation))
  (bind _dropspeed (Variables|Default|GetDropSpeed))
  (bind _outinstancetransform (Components|InstancedStaticMesh|GetInstanceTransform _instancecomponent _instanceid false))
  (bind (_location _rotation _scale) (Math|Transform|BreakTransform _outinstancetransform))
  (bind _returnvalue_2 (Math|Interpolation|VInterpTo _location _targetlocation _returnvalue _dropspeed))
  ;[0 0 0 0.5] This component allows you to instance the animation of each ISM instance, so you can loop through and perform a vertical movement and each one plays out independantly. The component is fire and forget, destroying itself once complete
  (Utilities|FlowControl|Gate true) ; enters at Close
)

(event Custom|OpenTickGate
  (bind _returnvalue (Utilities|Time|GetWorldDeltaSeconds))
  (bind _instanceid (Variables|Default|GetInstanceID))
  (bind _instancecomponent (Variables|Default|GetInstanceComponent))
  (bind _targetlocation (Variables|Default|GetTargetLocation))
  (bind _dropspeed (Variables|Default|GetDropSpeed))
  (bind _outinstancetransform (Components|InstancedStaticMesh|GetInstanceTransform _instancecomponent _instanceid false))
  (bind (_location _rotation _scale) (Math|Transform|BreakTransform _outinstancetransform))
  (bind _returnvalue_2 (Math|Interpolation|VInterpTo _location _targetlocation _returnvalue _dropspeed))
  ;[0 0 0 0.5] This component allows you to instance the animation of each ISM instance, so you can loop through and perform a vertical movement and each one plays out independantly. The component is fire and forget, destroying itself once complete
  (Utilities|FlowControl|Gate true) ; enters at Open
)

(event EventBeginPlay
  ;[0 0 0 0.5] This component allows you to instance the animation of each ISM instance, so you can loop through and perform a vertical movement and each one plays out independantly. The component is fire and forget, destroying itself once complete
  (Utilities|FlowControl|Delay 0.0) ; Expose on spawn variables do not get always set in time, so a 1 frame delay fixes this
  (Variables|Default|SetStartTransform (.location (.OutInstanceTransform (Components|InstancedStaticMesh|GetInstanceTransform (Variables|Default|GetInstanceComponent) (Variables|Default|GetInstanceID) false)))) ; Store Start Transform
  (Variables|Default|SetTargetLocation (- (Variables|Default|GetStartTransform) (Math|Vector|MakeVector 0.0 0.0 (Variables|Default|GetStartHeightToDrop)))) ; Store Desired Location
  (CallFunction|OpenTickGate))

(event EventTick
  (params (DeltaSeconds :type Float%20%28single-precision%29))
  (bind _returnvalue (Utilities|Time|GetWorldDeltaSeconds))
  (bind _instanceid (Variables|Default|GetInstanceID))
  (bind _instancecomponent (Variables|Default|GetInstanceComponent))
  (bind _targetlocation (Variables|Default|GetTargetLocation))
  (bind _dropspeed (Variables|Default|GetDropSpeed))
  (bind _outinstancetransform (Components|InstancedStaticMesh|GetInstanceTransform _instancecomponent _instanceid false))
  (bind (_location _rotation _scale) (Math|Transform|BreakTransform _outinstancetransform))
  (bind _returnvalue_2 (Math|Interpolation|VInterpTo _location _targetlocation _returnvalue _dropspeed))
  ;[0 0 0 0.5] This component allows you to instance the animation of each ISM instance, so you can loop through and perform a vertical movement and each one plays out independantly. The component is fire and forget, destroying itself once complete
  (Utilities|FlowControl|Gate true ; Allow tick once variables start and target have been saved
    (:Exit
      (Components|InstancedStaticMesh|UpdateInstanceTransform (Variables|Default|GetInstanceComponent) (Variables|Default|GetInstanceID) (Math|Transform|MakeTransform _returnvalue_2 _rotation _scale) false true false)
      (if (Math|Vector|Equal(Vector) _returnvalue_2 (Variables|Default|GetTargetLocation) 0.01) ; self destroy once interp has completed
        (CallFunction|CloseTickGate)
        (Default|CallMoveComplete) ; Optional dispatcher if needed
        (Components|DestroyComponent)))))